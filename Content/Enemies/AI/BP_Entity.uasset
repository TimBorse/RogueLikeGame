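; BP_Entity is a character Blueprint for enemies that holds health and movement speed and dies when health runs out.
; The construction script copies MovementSpeed into the character movement's max walk speed and fills HP from MaxHp.
; TakeDamage subtracts from HP, printing the remaining value while it stays above zero and otherwise calling KillCharacter, which destroys the actor.
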(fn ConstructionScript
  (Variables|/Script/Engine.CharacterMovementComponent|SetMaxWalkSpeed (Variables|Character|GetCharacterMovement) (Variables|Default|GetMovementSpeed))
  (Variables|Default|SetHP (Variables|Default|GetMaxHp)))

(fn TakeDamage
  (params (Amount :type Float%20%28double-precision%29))
  (bind _output_get (Variables|Default|SetHP (- (Variables|Default|GetHP) Amount)))
  (if (<= _output_get 0.0)
    (CallFunction|KillCharacter)
    (else
      (Development|PrintString (Utilities|String|ToString(Float) _output_get)))))

(fn KillCharacter
  (Actor|DestroyActor))