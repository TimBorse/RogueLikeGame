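; Enemy spawn point actor that spawns waves of simple melee enemies around itself.
; On BeginPlay it binds SpawnEnemy to the first-person game mode's next-wave event.
; Each wave spawns as many enemies as the wave number, with movement speed rising per wave and fixed damage, then increments the counter.
; Spawn locations are random reachable navmesh points, re-rolled until they lie beyond a minimum distance from the actor.
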(event Custom|Spawn%20Enemy
  (for _index (range 1 (Variables|Default|GetWave))
    (bind _randomlocation (CallFunction|GetRandomPointinRadiuswithMinDistance 5e+03 2e+03))
    (bind _returnvalue (Game|SpawnActorfromClass "/Game/Entities/Characters/Enemies/BP_Entity_SimpleMeele.BP_Entity_SimpleMeele_C" _randomlocation "AdjustIfPossibleButAlwaysSpawn" 0 0))
    (Default|SetMovementSpeed _returnvalue (+ (Variables|/Game/Entities/Characters/BP_Entity.BP_Entity_C|GetMovementSpeed _returnvalue) (* (Variables|Default|GetWave) 100)))
    (Variables|/Game/Entities/Characters/Enemies/BP_Entity_SimpleMeele.BP_Entity_SimpleMeele_C|SetDamage _returnvalue 1e+01))
  (bind _result (Math|Integer|IncrementInt (Variables|Default|GetWave))
    (:%20%20
      (Variables|Default|SetWave _result))))

(event EventBeginPlay
  (bind _asbp_first_person_game_mode (Utilities|Casting|CastToBP_FirstPersonGameMode (Game|GetGameMode)))
  (EventDispatchers|BindEventtoNextWave _asbp_first_person_game_mode (delegate Custom|Spawn%20Enemy)))

(fn ConstructionScript)

(fn GetRandomPointinRadiuswithMinDistance
  (params (Radius :type Float%20%28double-precision%29) (MinDistance :type Float%20%28double-precision%29))
  (bind _returnvalue (Transformation|GetActorLocation))
  (bind _randomlocation (AI|Navigation|GetRandomReachablePointinRadius _returnvalue Radius 0 0))
  ;[1 1 1] Gets random location in relation to actors location
  (LocalVariables|SetRandomLoc _randomlocation)
  (while (< (Math|Vector|Distance(Vector) (LocalVariables|GetRandomLoc) _returnvalue) MinDistance)
    (LocalVariables|SetRandomLoc _randomlocation))
  (return (Math|Conversions|ToTransform(Vector) (LocalVariables|GetRandomLoc))))