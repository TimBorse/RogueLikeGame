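; A simple melee enemy entity that damages the player on contact and registers itself in the game mode's living-enemy count.
; Tick checks the Box for player overlap, applies damage, then disables ticking for the damage cooldown so hits are spaced out.
; BeginPlay increments EnemiesAlive on the FirstPerson game mode, and the KillCharacter override decrements it and calls CheckEnemyLeft.
; A separate MakeDamage function calls TakeDamage on BP_Entity targets.
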(event EventBeginPlay
  (bind _asbp_first_person_game_mode (Utilities|Casting|CastToBP_FirstPersonGameMode (Game|GetGameMode)))
  (bind _result (Math|Integer|IncrementInt (Variables|/Game/FirstPerson/Blueprints/BP_FirstPersonGameMode.BP_FirstPersonGameMode_C|GetEnemiesAlive _asbp_first_person_game_mode))
    (:%20%20
      (Variables|/Game/FirstPerson/Blueprints/BP_FirstPersonGameMode.BP_FirstPersonGameMode_C|SetEnemiesAlive _asbp_first_person_game_mode _result))))

(event EventTick
  (params (DeltaSeconds :type Float%20%28single-precision%29))
  (bind _returnvalue (Game|GetPlayerCharacter 0))
  ;[1 1 1] Check for collision each tick, when collided with player the ticking gets paused to 1 second so the player does not die instantly
  (if (Collision|IsOverlappingActor (Variables|Default|GetBox) _returnvalue :!class /Script/Engine.PrimitiveComponent)
    (bind _asbp_first_person_character (Utilities|Casting|CastToBP_FirstPersonCharacter _returnvalue))
    (Game|Damage|ApplyDamage _asbp_first_person_character (Variables|Default|GetDamage) 0 0)
    (Actor|Tick|SetActorTickEnabled false)
    (Utilities|FlowControl|Delay (Variables|Default|GetDamageCooldown))
    (Actor|Tick|SetActorTickEnabled true)))

(fn ConstructionScript
  (|CallParentFunction))

(fn MakeDamage
  (params (Target :type Actor%20Object%20Reference))
  (bind _asbp_entity (Utilities|Casting|CastToBP_Entity Target)
    (:then
      (Default|TakeDamage _asbp_entity (Variables|Default|GetDamage)))
    (:CastFailed
      (Development|PrintString "Failed!"))))

(fn KillCharacter
  (|CallParentFunction)
  (bind _asbp_first_person_game_mode (Utilities|Casting|CastToBP_FirstPersonGameMode (Game|GetGameMode)))
  (bind _result (Math|Integer|DecrementInt (Variables|/Game/FirstPerson/Blueprints/BP_FirstPersonGameMode.BP_FirstPersonGameMode_C|GetEnemiesAlive _asbp_first_person_game_mode))
    (:%20%20
      (Variables|/Game/FirstPerson/Blueprints/BP_FirstPersonGameMode.BP_FirstPersonGameMode_C|SetEnemiesAlive _asbp_first_person_game_mode _result)
      (Default|CheckEnemyLeft _asbp_first_person_game_mode))))