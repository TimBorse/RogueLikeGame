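; Simple melee enemy entity that damages the first-person player character on contact.
; Each tick it checks whether its Box overlaps the player and, if so, applies Damage.
; It then disables its own ticking for DamageCooldown, throttling hits so the player does not die instantly.
; A separate MakeDamage function, not called in these graphs, calls TakeDamage on BP_Entity targets.
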(event EventTick
  (params (DeltaSeconds :type Float%20%28single-precision%29))
  (bind _returnvalue (Game|GetPlayerCharacter 0))
  ;[1 1 1] Check for collision each tick, when collided with player the ticking gets paused to 1 second so the player does not die instantly
  (if (Collision|IsOverlappingActor (Variables|Default|GetBox) _returnvalue :!class /Script/Engine.PrimitiveComponent)
    (bind _asbp_first_person_character (Utilities|Casting|CastToBP_FirstPersonCharacter _returnvalue))
    (Game|Damage|ApplyDamage _asbp_first_person_character (Variables|Default|GetDamage) 0 0)
    (Actor|Tick|SetActorTickEnabled false)
    (Utilities|FlowControl|Delay (Variables|Default|GetDamageCooldown))
    (Actor|Tick|SetActorTickEnabled true)))

(fn ConstructionScript
  (|CallParentFunction))

(fn MakeDamage
  (params (Target :type Actor%20Object%20Reference))
  (bind _asbp_entity (Utilities|Casting|CastToBP_Entity Target)
    (:then
      (Default|TakeDamage _asbp_entity (Variables|Default|GetDamage)))
    (:CastFailed
      (Development|PrintString "Failed!"))))