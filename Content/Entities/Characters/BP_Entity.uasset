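; BP_Entity is a character Blueprint that provides health, movement speed and death handling.
; Construction sets walk speed and fills HP from its maximum, and SetMovementSpeed updates the speed later.
; AnyDamage feeds TakeDamage, which clamps HP and either prints it or calls KillCharacter at zero.
; KillCharacter destroys the actor and spawns a fire emitter, whose component it destroys immediately.
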(event Game|Damage|EventAnyDamage
  (params (Damage :type Float%20%28single-precision%29) (DamageType :type Damage%20Type%20Object%20Reference) (InstigatedBy :type Controller%20Object%20Reference) (DamageCauser :type Actor%20Object%20Reference))
  (CallFunction|TakeDamage Damage))

(fn ConstructionScript
  (Variables|/Script/Engine.CharacterMovementComponent|SetMaxWalkSpeed (Variables|Character|GetCharacterMovement) (Variables|Default|GetMovementSpeed))
  (Variables|Default|SetHP (Variables|Default|GetMaxHp)))

(fn TakeDamage
  (params (Amount :type Float%20%28double-precision%29))
  (bind _output_get (Variables|Default|SetHP (Math|Float|Clamp(Float) (- (Variables|Default|GetHP) Amount) 0.0 (Variables|Default|GetMaxHp))))
  (if (<= _output_get 0.0)
    (CallFunction|KillCharacter)
    (else
      (Development|PrintString (Utilities|String|ToString(Float) _output_get)))))

(fn KillCharacter
  (Actor|DestroyActor)
  (bind _returnvalue (Effects|SpawnEmitteratLocation "/Game/_Init/StarterContent/Particles/P_Fire.P_Fire" "0, 0, 0"))
  (Components|DestroyComponent _returnvalue))

(fn SetMovementSpeed
  (params (New%20Movementspeed :type Float%20%28double-precision%29))
  (bind _output_get (Variables|Default|SetMovementSpeed New%20Movementspeed))
  (Variables|/Script/Engine.CharacterMovementComponent|SetMaxWalkSpeed (Variables|Character|GetCharacterMovement) _output_get))