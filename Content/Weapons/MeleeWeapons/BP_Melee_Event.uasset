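; BP_Melee_Event is an animation notify state that marks the active attack window of a melee animation for the first-person character.
; On begin, it casts the mesh owner to BP_FirstPersonCharacter and its right-hand weapon component to BP_Skeletal_Melee_Weapon_Component, then calls TriggerMeleeWeapon.
; On end, it repeats the same lookup and calls StopMeleeAttack, doing nothing if either cast fails.
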(fn ReceivedNotifyBegin
  (params (MeshComp :type Skeletal%20Mesh%20Component%20Object%20Reference) (Animation :type Anim%20Sequence%20Base%20Object%20Reference) (TotalDuration :type Float%20%28single-precision%29) (EventReference :type Anim%20Notify%20Event%20Reference%20Structure%20%28by%20ref%29))
  (bind _asbp_first_person_character (Utilities|Casting|CastToBP_FirstPersonCharacter (Components|GetOwner MeshComp)))
  (bind _asbp_skeletal_melee_weapon_component (Utilities|Casting|CastToBP_Skeletal_Melee_Weapon_Component (Variables|/Game/Entities/Characters/Player/BP_FirstPersonCharacter.BP_FirstPersonCharacter_C|GetRightHandWeaponComponent _asbp_first_person_character)))
  (Default|TriggerMeleeWeapon _asbp_skeletal_melee_weapon_component)
  (return false))

(fn ReceivedNotifyEnd
  (params (MeshComp :type Skeletal%20Mesh%20Component%20Object%20Reference) (Animation :type Anim%20Sequence%20Base%20Object%20Reference) (EventReference :type Anim%20Notify%20Event%20Reference%20Structure%20%28by%20ref%29))
  (bind _asbp_first_person_character (Utilities|Casting|CastToBP_FirstPersonCharacter (Components|GetOwner MeshComp)))
  (bind _asbp_skeletal_melee_weapon_component (Utilities|Casting|CastToBP_Skeletal_Melee_Weapon_Component (Variables|/Game/Entities/Characters/Player/BP_FirstPersonCharacter.BP_FirstPersonCharacter_C|GetRightHandWeaponComponent _asbp_first_person_character)))
  (Default|StopMeleeAttack _asbp_skeletal_melee_weapon_component)
  (return false))