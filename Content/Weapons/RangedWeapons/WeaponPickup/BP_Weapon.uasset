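; BP_Weapon is a weapon pickup that equips the first-person character when it overlaps the pickup's sphere.
; On overlap it adds a BP skeletal weapon component to the character, passes it the weapon class, skeletal mesh and shoot interval as cooldown, then destroys itself.
; The construction script applies the same mesh to the Sword component, so the placed pickup displays the weapon it grants.
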(event OnComponentBeginOverlap(Sphere)
  (params (OverlappedComponent :type Primitive%20Component%20Object%20Reference) (OtherActor :type Actor%20Object%20Reference) (OtherComp :type Primitive%20Component%20Object%20Reference) (OtherBodyIndex :type Integer) (bFromSweep :type Boolean) (SweepResult :type Hit%20Result%20Structure%20%28by%20ref%29))
  (bind _asbp_first_person_character (Utilities|Casting|CastToBP_FirstPersonCharacter OtherActor))
  (bind _output_get (Variables|Default|SetAs%20BP%20First%20Person%20Character_1 _asbp_first_person_character))
  (bind _returnvalue (AddComponent|AddBPSkeletalWeaponComponent _output_get false))
  (Variables|/Game/Weapons/RangedWeapons/WeaponComponent/BP_Skeletal_Weapon_Component.BP_Skeletal_Weapon_Component_C|SetWeaponClass _returnvalue (Variables|Default|GetWeapon%20Class))
  (Components|SkeletalMesh|SetSkeletalMeshAsset _returnvalue (Variables|Default|GetSkeletonMesh))
  (Variables|/Game/Weapons/RangedWeapons/WeaponComponent/BP_Skeletal_Weapon_Component.BP_Skeletal_Weapon_Component_C|SetCooldown _returnvalue (Variables|Default|GetShootInterval))
  (Actor|DestroyActor))

(fn ConstructionScript
  (Components|SkeletalMesh|SetSkeletalMeshAsset (Variables|Default|GetSword) (Variables|Default|GetSkeletonMesh)))